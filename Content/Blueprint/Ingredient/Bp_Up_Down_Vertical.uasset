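; Ingredient actor whose Cube1 component steps up or down vertically when a Bp_Boulette overlaps one of its trigger boxes.
; An overlap with BoxUp raises Cube1 and one with Box lowers it by the same fixed world-space offset.
; Each move is an instant, unswept location change with no interpolation or limit on travel.
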(event OnComponentBeginOverlap(BoxUp)
  (params (OverlappedComponent :type Primitive%20Component%20Object%20Reference) (OtherActor :type Actor%20Object%20Reference) (OtherComp :type Primitive%20Component%20Object%20Reference) (OtherBodyIndex :type Integer) (bFromSweep :type Boolean) (SweepResult :type Hit%20Result%20Structure%20%28by%20ref%29))
  (bind _cube1 (Variables|Default|GetCube1))
  (Utilities|Casting|CastToBp_Boulette OtherActor)
  (Transformation|SetWorldLocation _cube1 (+ (Transformation|GetWorldLocation _cube1) "0, 0,25.000000") false false))

(event OnComponentBeginOverlap(Box)
  (params (OverlappedComponent :type Primitive%20Component%20Object%20Reference) (OtherActor :type Actor%20Object%20Reference) (OtherComp :type Primitive%20Component%20Object%20Reference) (OtherBodyIndex :type Integer) (bFromSweep :type Boolean) (SweepResult :type Hit%20Result%20Structure%20%28by%20ref%29))
  (bind _cube1 (Variables|Default|GetCube1))
  (Utilities|Casting|CastToBp_Boulette OtherActor)
  (Transformation|SetWorldLocation _cube1 (+ (Transformation|GetWorldLocation _cube1) "0, 0,-25.000000") false false))

(fn ConstructionScript)