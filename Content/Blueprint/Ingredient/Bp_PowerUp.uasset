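; Bp_PowerUp is a pickup that grants an ability to the Bp_Larry_A character when it overlaps the Box component.
; Boolean flags select the power: bazooka sets the character's IsBazooka, and double jump raises or lowers its JumpAdd to a fixed value.
; Both of these branches destroy the pickup, while the wall jump flag is checked but has no effect.
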(event OnComponentBeginOverlap(Box)
  (params (OverlappedComponent :type Primitive%20Component%20Object%20Reference) (OtherActor :type Actor%20Object%20Reference) (OtherComp :type Primitive%20Component%20Object%20Reference) (OtherBodyIndex :type Integer) (bFromSweep :type Boolean) (SweepResult :type Hit%20Result%20Structure%20%28by%20ref%29))
  (bind _asbp_larry_a (Utilities|Casting|CastToBp_Larry_A OtherActor))
  (Utilities|FlowControl|Sequence
    (:then_0
      (if (Variables|Default|GetisBazooka)
        (Variables|/Game/Blueprint/Character/Bp_Larry_A.Bp_Larry_A_C|SetisBazooka _asbp_larry_a true)
        (Actor|DestroyActor :!label _label)))
    (:then_1
      (if (Variables|Default|GetisDoubleJump)
        (Variables|/Game/Blueprint/Character/Bp_Larry_A.Bp_Larry_A_C|SetJumpAdd _asbp_larry_a 2)
        (goto _label)))
    (:then_2
      (if (Variables|Default|GetisWalljump)
        _))))

(fn ConstructionScript)