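; Larry, the Paper2D side-scrolling player character with run, stand-still, double jump, trace-based wall jump and shooting; dash is unfinished.
; Tick turns the controller to face movement, picks flipbooks from walk/idle/shoot flags and aims an arrow from axis input.
; The arrow spawns Bp_Boulette projectiles, repeating at a delayed rate in bazooka mode.
; Boss bullets drain Mojo; depletion triggers an explosion, death widget and checkpoint teleport.
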(event OnComponentBeginOverlap(Box)
  (params (OverlappedComponent :type Primitive%20Component%20Object%20Reference) (OtherActor :type Actor%20Object%20Reference) (OtherComp :type Primitive%20Component%20Object%20Reference) (OtherBodyIndex :type Integer) (bFromSweep :type Boolean) (SweepResult :type Hit%20Result%20Structure%20%28by%20ref%29))
  (Utilities|Casting|CastToBp_BouletteBoss OtherActor)
  (Development|PrintString "Ouch!!!")
  (CallFunction|MojoFunction 1e+01))

(event Custom|WallJump
  (bind _returnvalue (Transformation|GetActorForwardVector))
  ;[0.05208 0.05208 0.05208] Wall Jump and double Jump : https://www.youtube.com/watch?v=lV558lay89k
  ;;[1 1 1] WallJump
  (bind (_outhit _returnvalue_2) (Collision|LineTraceByChannel (- (Transformation|GetActorLocation) (* _returnvalue (+ (Components|Capsule|GetScaledCapsuleRadius (Variables|Collision|GetCapsuleComponent)) 15.0))) (+ (Transformation|GetActorLocation) (* _returnvalue (+ (Components|Capsule|GetScaledCapsuleRadius (Variables|Collision|GetCapsuleComponent)) 15.0))) "TraceTypeQuery1" true 0 "None"))
  (if _returnvalue_2
    (Character|LaunchCharacter (Math|Vector|MakeVector (* (Math|Float|Sign(Float) (- (.x (Transformation|GetActorLocation)) (.x (.Location (Collision|BreakHitResult _outhit))))) 1.5e+03) 0.0 (* (Variables|/Script/Engine.CharacterMovementComponent|GetJumpZVelocity (Variables|Character|GetCharacterMovement)) 3.0)) true true)
    (elif (<= (Variables|Default|GetJumpCount) 2)
      (Character|Jump)
      (Variables|Default|SetJumpCount (+ (Variables|Default|GetJumpCount) 1)))))

(event Custom|UpdateAnimation
  ;[0.0918 1 0] Handle Animation
  (Sprite|SetFlipbook (Variables|Default|GetSprite) (select (> (Math|Vector|VectorLength (Transformation|GetVelocity)) 0.0) "/Game/Proto/2DSideScroller/Sprites/RunningAnimation.RunningAnimation" "/Game/Proto/2DSideScroller/Sprites/IdleAnimation.IdleAnimation")))

(event Custom|DeathTick
  ;[0.2448 0.004628 0] DEath
  (Utilities|FlowControl|Sequence
    (:then_0
      (if (Variables|Default|GetisDead)
        (Utilities|FlowControl|DoOnce false :!label _label
          (:Completed
            (bind _output_get (Variables|Default|SetExplosionLocation (Transformation|GetWorldLocation (Variables|Collision|GetCapsuleComponent))))
            (Effects|SpawnEmitteratLocation "/Game/Proto/StarterContent/Particles/P_Explosion.P_Explosion" _output_get)
            (bind _returnvalue (UserInterface|CreateWidget "/Game/HUD/Widget/Death_Widget.Death_Widget_C"))
            (UserInterface|Viewport|AddtoViewport _returnvalue 0)
            (Utilities|FlowControl|Delay 0.5)
            (Transformation|Teleport self (Variables|Default|GetLastCheckpoint) "0, 0, 0")
            (Variables|Default|SetisDead false)
            (Utilities|FlowControl|Delay 2.0)
            (Widget|RemovefromParent _returnvalue)
            (goto _label Reset)))))
    (:then_1
      (if (<= (Variables|Default|GetMojo) 0.0)
        (Variables|Default|SetisDead true)
        (Utilities|FlowControl|Delay 0.2)
        (Variables|Default|SetisDead false)
        (Variables|Default|SetMojo 1e+02)))))

(event EventOnLanded
  (params (Hit :type Hit%20Result%20Structure%20%28by%20ref%29))
  ;[0.05208 0.05208 0.05208] Wall Jump and double Jump : https://www.youtube.com/watch?v=lV558lay89k
  ;;[1 1 1] Landed
  (Variables|Default|SetJumpCount 0))

(event EventTick
  (params (DeltaSeconds :type Float%20%28single-precision%29))
  (bind _returnvalue (Game|GetPlayerCharacter 0))
  (bind _idle_anim_larry (Variables|Default|GetIdle_Anim_Larry))
  (bind _returnvalue_2 (Transformation|GetActorLocation _returnvalue))
  ;[1 0 0.01752] Tick
  (Utilities|FlowControl|Sequence
    (:then_0
      ;[1 1 1] Tick - Updates animation
      (CallFunction|UpdateAnimation)
      (Math|Float|CompareFloat (.X (Math|Vector|BreakVector (Variables|/Script/Engine.MovementComponent|GetVelocity (Pawn|GetMovementComponent)))) 0.0
        (:>
          (Pawn|SetControlRotation (Pawn|GetController) (Math|Rotator|MakeRotator 0.0 0.0 0.0) :!label _label))
        (:==
          (if (Variables|Default|GetbisMovingRight)
            (goto _label)
            (else
              (Pawn|SetControlRotation (Pawn|GetController) (Math|Rotator|MakeRotator 0.0 0.0 1.8e+02) :!label _label_2))))
        (:<
          (goto _label_2))))
    (:then_1
      ;[1 1 1] anim
      (Utilities|FlowControl|Sequence
        (:then_0
          (if (Variables|Default|GetisShoot)
            (Sprite|SetFlipbook _idle_anim_larry "/Game/2DArt/Laurent2D/Larry/Shoot_Anim_Larry1.Shoot_Anim_Larry1")
            (elif (Variables|Default|GetisIdle)
              (Sprite|SetFlipbook _idle_anim_larry "/Game/2DArt/Laurent2D/Larry/Idle_Anim_Larry.Idle_Anim_Larry" :!label _label_3))))
        (:then_2
          (if (Variables|Default|GetisWalk)
            (if (Variables|Default|GetisStandStill)
              (goto _label_3)
              (else
                (Sprite|SetFlipbook _idle_anim_larry "/Game/2DArt/Laurent2D/Larry/Walk_Anim_Larry2.Walk_Anim_Larry2")))))))
    (:then_2
      ;[1 0.1073 0.02767] BouletteAxis
      (Utilities|FlowControl|Sequence
        (:then_1
          (Variables|Default|SetisAxisMoving (and (== (stale Input|AxisEvents|InputAxisGaucheDroite AxisValue) 0.0) (== (stale Input|AxisEvents|InputAxisHautBas AxisValue) 0.0)))
          (if (not (and (== (stale Input|AxisEvents|InputAxisGaucheDroite AxisValue) 0.0) (== (stale Input|AxisEvents|InputAxisHautBas AxisValue) 0.0)))
            (Transformation|SetWorldRotation (Variables|Default|GetArrow1) (Math|Rotator|FindLookatRotation (+ (Math|Vector|MakeVector (stale Input|AxisEvents|InputAxisGaucheDroite AxisValue) 0.0 (stale Input|AxisEvents|InputAxisHautBas AxisValue)) _returnvalue_2) _returnvalue_2) false false)))
        (:then_2
          (Variables|Default|SetArrowLock (stale Input|AxisEvents|InputAxisHautBas AxisValue)))))
    (:then_3
      (if (Variables|Default|GetisBazooka)
        (if (Variables|Default|GetCanShoot)
          (Utilities|FlowControl|Delay (Variables|Default|GetROF))
          (bind _returnvalue_3 (Game|SpawnActorfromClass "/Game/Blueprint/Boulette/Bp_Boulette.Bp_Boulette_C" (Transformation|GetWorldTransform (Variables|Default|GetArrow1)) "Undefined" 0 0))
          (Variables|Default|SetisIdle false)
          (Variables|Default|SetisShoot true)
          (Variables|Default|SetisWalk false)
          (Utilities|FlowControl|Delay 0.3)
          (Variables|Default|SetisShoot false)
          (Variables|Default|SetisIdle true)
          (Variables|Default|SetisWalk false))))
    (:then_4
      (CallFunction|DeathTick))
    (:then_6
      (Development|PrintString (Utilities|String|ToString(Rotator) (Transformation|GetWorldRotation (Variables|Default|GetArrow1))) true true "(R=0.000000,G=0.660000,B=1.000000,A=1.000000)" 0.01))))

(event EventBeginPlay
  (Class|ActorComponent|SetIsReplicated (Variables|Default|GetSprite) true))

(event Input|ActionEvents|InputActionDashLeft
  (params (Key :type Key%20Structure))
  ;[1 0 0.7564] Dash to come
)

(event Input|ActionEvents|InputActionStandStill
  (params (Key :type Key%20Structure))
  (bind _charactermovement (Variables|Character|GetCharacterMovement))
  ;[0 0 0] Stop Walk Trigger
  (:Pressed
    (Variables|/Script/Engine.CharacterMovementComponent|SetMaxWalkSpeed _charactermovement 0.0)
    (Variables|Default|SetisStandStill true))
  (:Released
    (Variables|/Script/Engine.CharacterMovementComponent|SetMaxWalkSpeed _charactermovement 5e+02)
    (Variables|Default|SetisStandStill false)))

(event Input|ActionEvents|InputActionRun
  (params (Key :type Key%20Structure))
  (bind _charactermovement (Variables|Character|GetCharacterMovement))
  ;[1 1 1] Run
  (:Pressed
    (Variables|/Script/Engine.CharacterMovementComponent|SetMaxWalkSpeed _charactermovement 1.2e+03))
  (:Released
    (Variables|/Script/Engine.CharacterMovementComponent|SetMaxWalkSpeed _charactermovement 5e+02)))

(event Input|ActionEvents|InputActionShoot
  (params (Key :type Key%20Structure))
  ;[1 0.1073 0.02767] BouletteAxis
  (:Pressed
    (Variables|Default|SetCanShoot true)
    (if (Variables|Default|GetisBazooka)
      (if (Variables|Default|GetCanShoot)
        (Utilities|FlowControl|Delay (Variables|Default|GetROF))
        (bind _returnvalue (Game|SpawnActorfromClass "/Game/Blueprint/Boulette/Bp_Boulette.Bp_Boulette_C" (Transformation|GetWorldTransform (Variables|Default|GetArrow1)) "Undefined" 0 0 :!label _label))
        (Variables|Default|SetisIdle false)
        (Variables|Default|SetisShoot true)
        (Variables|Default|SetisWalk false)
        (Utilities|FlowControl|Delay 0.3)
        (Variables|Default|SetisShoot false)
        (Variables|Default|SetisIdle true)
        (Variables|Default|SetisWalk false))
      (else
        (goto _label))))
  (:Released
    (Variables|Default|SetCanShoot false)))

(event Input|ActionEvents|InputActionDashRight
  (params (Key :type Key%20Structure))
  ;[1 0 0.7564] Dash to come
)

(event Input|ActionEvents|InputActionJump
  (params (Key :type Key%20Structure))
  ;[0.05208 0.05208 0.05208] Wall Jump and double Jump : https://www.youtube.com/watch?v=lV558lay89k
  ;;[1 1 1] Handle Jump
  (:Pressed
    (Character|Jump)
    (if (AI|Components|NavMovement|IsFalling (Variables|Character|GetCharacterMovement))
      (CallFunction|WallJump)
      (Variables|Default|SetJumpCount 0)
      (else
        (Character|Jump)
        (Variables|Default|SetJumpCount (+ (Variables|Default|GetJumpCount) 1)))))
  (:Released
    (if (>= (Math|Conversions|ToByte(Integer) (Variables|Default|GetJumpCount)) (Math|Conversions|ToByte(Integer) (Variables|Default|GetJumpAdd)))
      (Character|StopJumping))))

(event Input|AxisEvents|InputAxisGaucheDroite
  (params (AxisValue :type Float%20%28single-precision%29))
  ;[1 0.1073 0.02767] BouletteAxis
)

(event Input|AxisEvents|InputAxisHautBas
  (params (AxisValue :type Float%20%28single-precision%29))
  ;[1 0.1073 0.02767] BouletteAxis
)

(event Input|AxisEvents|InputAxisMoveRight
  (params (AxisValue :type Float%20%28single-precision%29))
  ;[1 1 1] Handle movement
  (if (> AxisValue 0.95)
    (Variables|Default|SetbisMovingRight true)
    (Utilities|FlowControl|Sequence
      (:then_0
        (Pawn|Input|AddMovementInput "1.000000, 0, 0" AxisValue false :!label _label))
      (:then_1
        (Variables|Default|SetisWalk true)
        (Variables|Default|SetisShoot false)
        (Variables|Default|SetisIdle false)
        (Utilities|FlowControl|RetriggerableDelay 1.0)
        (Variables|Default|SetisWalk false)
        (Variables|Default|SetisShoot false)
        (Variables|Default|SetisIdle true)))
    (elif (< AxisValue -0.95)
      (Variables|Default|SetbisMovingRight false)
      (Variables|Default|SetisWalk true)
      (Variables|Default|SetisShoot false)
      (Variables|Default|SetisIdle false)
      (goto _label)
      (else
        (Utilities|FlowControl|Sequence
          (:then_0
            (goto _label))
          (:then_1
            (if (not (Variables|Default|GetisShoot))
              (Variables|Default|SetisWalk false)
              (Variables|Default|SetisShoot false)
              (Variables|Default|SetisIdle true))))))))

(event Input|TouchEvents|InputTouch
  (params (Location :type Vector) (FingerIndex :type ETouchIndex%20Enum))
  ;[0.05208 0.05208 0.05208] Wall Jump and double Jump : https://www.youtube.com/watch?v=lV558lay89k
  ;;[1 1 1] Handle Jump
)

(fn ConstructionScript
  (Variables|/Script/Engine.CharacterMovementComponent|SetJumpZVelocity (Variables|Character|GetCharacterMovement) 6e+02)
  (Variables|Default|SetJumpMaxHoldTime 0.4)
  (Variables|Default|SetJumpCount 0))

(fn ShootFunction)

(fn MojoFunction
  (params (Hp :type Float%20%28single-precision%29))
  (Variables|Default|SetMojo (- (Variables|Default|GetMojo) Hp)))