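; CameraDistance is a trigger volume actor meant to change the Bp_Larry_A character's camera boom distance.
; When Larry leaves the Box, the boom's TargetArmLength snaps to DistanceCamOut.
; Entering only enables the actor's tick, which is empty.
; The DistanceCam arm length, target offset changes, view target blend and interpolation nodes are disconnected, so no zoom applies on entry.
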(event OnComponentBeginOverlap(Box)
  (params (OverlappedComponent :type Primitive%20Component%20Object%20Reference) (OtherActor :type Actor%20Object%20Reference) (OtherComp :type Primitive%20Component%20Object%20Reference) (OtherBodyIndex :type Integer) (bFromSweep :type Boolean) (SweepResult :type Hit%20Result%20Structure%20%28by%20ref%29))
  (bind _asbp_larry_a (Utilities|Casting|CastToBp_Larry_A OtherActor))
  (Actor|Tick|SetActorTickEnabled true))

(event OnComponentEndOverlap(Box)
  (params (OverlappedComponent :type Primitive%20Component%20Object%20Reference) (OtherActor :type Actor%20Object%20Reference) (OtherComp :type Primitive%20Component%20Object%20Reference) (OtherBodyIndex :type Integer))
  (bind _asbp_larry_a (Utilities|Casting|CastToBp_Larry_A OtherActor))
  (Variables|/Script/Engine.SpringArmComponent|SetTargetArmLength (Variables|/Game/Blueprint/Character/Bp_Larry_A.Bp_Larry_A_C|GetCameraBoom _asbp_larry_a) (Variables|Default|GetDistanceCamOut)))

(event EventTick
  (params (DeltaSeconds :type Float%20%28single-precision%29)))

(fn ConstructionScript)